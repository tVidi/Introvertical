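; GM_Main is the main game mode, which triggers the game over screen when the player's social battery runs out.
; On BeginPlay it caches the GS_Main game state and binds to the OnDepleted event of PS_Player's SocialBattery.
; When depleted, TryShowEndScreen clears the game state's IsGameRunning flag and adds WBP_GameOver to the viewport, with that flag guarding against repeat triggers.
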(event `OnPlayerDepleted`
  (`self.TryShowEndScreen`))

(event `self.ReceiveBeginPlay`
  (bind _asgs_main (cast `/Game/Blueprints/Game/GS_Main` (`GameplayStatics.GetGameState`)))
  (set `self.As GS Main` _asgs_main)
  (bind _asps_player (cast `/Game/Blueprints/Characters/Player/PS_Player` (`GameplayStatics.GetPlayerState` 0)))
  (add `/Game/Blueprints/Components/AC_SocialBatteryComponent.OnDepleted` (`/Game/Blueprints/Characters/Player/PS_Player.SocialBattery` _asps_player) (delegate `OnPlayerDepleted`)))

(fn `TryShowEndScreen`
  (bind _as_gs_main (`self.As GS Main`))
  (if (`/Game/Blueprints/Game/GS_Main.bIsGameRunning` _as_gs_main)
    (set `/Game/Blueprints/Game/GS_Main.bIsGameRunning` false _as_gs_main)
    (bind _returnvalue (`|CreateWidget` "/Game/UI/Widgets/Menus/WBP_GameOver.WBP_GameOver_C" (`GameplayStatics.GetPlayerController` 0)))
    (`UserWidget.AddToViewport` _returnvalue 0)))

(fn `UserConstructionScript`)