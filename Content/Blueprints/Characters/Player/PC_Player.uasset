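; Player controller for a first-person character that adds the mapping context and forwards Enhanced Input to the possessed CHAR_Player.
; Look, move and jump pass straight through, while sprint toggles on a FlipFlop.
; Crouch also starts a slide, and releasing it, or triggering it while crouched, uncrouches and stops the slide.
; Tick ends a slide once horizontal speed falls to crouched walk speed or below.
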(event `self.ReceiveBeginPlay`
  (`EnhancedInputSubsystemInterface.AddMappingContext` (subsystem `EnhancedInputLocalPlayerSubsystem`) (`self.FirstPersonMapping`) 0 (struct))
  (bind _aschar_player (cast `/Game/Blueprints/Characters/Player/CHAR_Player` (`self.K2_GetPawn`)))
  (set `self.PlayerCharacter` _aschar_player))

(event `self.ReceiveTick`
  (params (DeltaSeconds :type "Float (single-precision)"))
  (bind _playercharacter (`self.PlayerCharacter`))
  (if (and (`/Game/Blueprints/Characters/Player/CHAR_Player.bIsSliding` _playercharacter) (<= (`/Game/Blueprints/Characters/Player/CHAR_Player.Get Horizontal Velocity (Float)` _playercharacter) (`CharacterMovementComponent.MaxWalkSpeedCrouched` (`Character.CharacterMovement` _playercharacter))))
    (`/Game/Blueprints/Characters/Player/CHAR_Player.StopSliding` (`self.PlayerCharacter`))))

(event `EnhancedInput|/Game/Data/Input/FirstPerson/IA_Look`
  (params (ActionValue :type "Vector2D Structure") (ElapsedSeconds :type "Float (double-precision)") (TriggeredSeconds :type "Float (double-precision)") (InputAction :type "InputAction Object Reference" :default "/Game/Data/Input/FirstPerson/IA_Look.IA_Look"))
  ;[0.4 0.8 0 0.2] Look
  (:`Triggered`
    (`/Game/Blueprints/Characters/Player/CHAR_Player.Look` (`self.PlayerCharacter`) ActionValue)))

(event `EnhancedInput|/Game/Data/Input/FirstPerson/IA_Move`
  (params (ActionValue :type "Vector2D Structure") (ElapsedSeconds :type "Float (double-precision)") (TriggeredSeconds :type "Float (double-precision)") (InputAction :type "InputAction Object Reference" :default "/Game/Data/Input/FirstPerson/IA_Move.IA_Move"))
  ;[0.4 0.8 0 0.2] Move, Sprint
  (:`Triggered`
    (`/Game/Blueprints/Characters/Player/CHAR_Player.Move` (`self.PlayerCharacter`) ActionValue)))

(event `EnhancedInput|/Game/Data/Input/FirstPerson/IA_Sprint`
  (params (ActionValue :type Boolean) (ElapsedSeconds :type "Float (double-precision)") (TriggeredSeconds :type "Float (double-precision)") (InputAction :type "InputAction Object Reference" :default "/Game/Data/Input/FirstPerson/IA_Sprint.IA_Sprint"))
  (bind _playercharacter (`self.PlayerCharacter`))
  ;[0.4 0.8 0 0.2] Move, Sprint
  (:`Triggered`
    (`/Engine/EditorBlueprintResources/StandardMacros.FlipFlop`
      (:`A`
        (`/Game/Blueprints/Characters/Player/CHAR_Player.Sprint` _playercharacter))
      (:`B`
        (`/Game/Blueprints/Characters/Player/CHAR_Player.StopSprinting` _playercharacter)))))

(event `EnhancedInput|/Game/Data/Input/FirstPerson/IA_Jump`
  (params (ActionValue :type Boolean) (ElapsedSeconds :type "Float (double-precision)") (TriggeredSeconds :type "Float (double-precision)") (InputAction :type "InputAction Object Reference" :default "/Game/Data/Input/FirstPerson/IA_Jump.IA_Jump"))
  ;[0.4 0.8 0 0.2] Jump, Crouch
  (:`Started`
    (`Character.Jump` (`self.PlayerCharacter`))))

(event `EnhancedInput|/Game/Data/Input/FirstPerson/IA_Crouch`
  (params (ActionValue :type Boolean) (ElapsedSeconds :type "Float (double-precision)") (TriggeredSeconds :type "Float (double-precision)") (InputAction :type "InputAction Object Reference" :default "/Game/Data/Input/FirstPerson/IA_Crouch.IA_Crouch"))
  (bind _playercharacter (`self.PlayerCharacter`))
  ;[0.4 0.8 0 0.2] Jump, Crouch
  (:`Triggered`
    (if (`Character.bIsCrouched` _playercharacter)
      (`Character.UnCrouch` _playercharacter :!label _label)
      (`/Game/Blueprints/Characters/Player/CHAR_Player.StopSliding` _playercharacter)
      (else
        (`Character.Crouch` _playercharacter)
        (`/Game/Blueprints/Characters/Player/CHAR_Player.Slide` _playercharacter) ; Sliding triggers OnLanded for some reason, likely due to the player being launched
      )))
  (:`Completed`
    (goto _label)))

(fn `UserConstructionScript`)