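; Actor component that tracks a social battery charge for its owner, starting at the maximum on BeginPlay.
; UpdateCharge adds a signed amount with no upper clamp, fires the OnUpdateCharge dispatcher and prints the new value for debugging.
; Reaching zero or below clamps the charge to zero and sets IsDead, which blocks all further updates.
; GetCharge and IsDepleted expose the current state.
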(event `self.ReceiveBeginPlay`
  (set `self.Charge` (`self.MaxCharge`)))

(fn `GetCharge`
  (returns (Charge :type "Float (double-precision)"))
  (return (`self.Charge`)))

(fn `IsDepleted`
  (returns (Result :type Boolean))
  (return (<= (`self.Charge`) 0.0)))

(fn `UpdateCharge`
  (params (Amount :type "Float (double-precision)"))
  (returns (Result :type "Float (double-precision)"))
  (bind _charge (`self.Charge`))
  (if (not (`self.IsDead`))
    (set `self.Charge` (+ Amount (`self.Charge`)))
    (bind _output_get (set `self.IsDead` (`self.IsDepleted`)))
    (if _output_get
      (set `self.Charge` 0.0))
    (`self.OnUpdateCharge`)
    (`KismetSystemLibrary.PrintString` (`KismetStringLibrary.Conv_DoubleToString` _charge))
    (return _charge)))